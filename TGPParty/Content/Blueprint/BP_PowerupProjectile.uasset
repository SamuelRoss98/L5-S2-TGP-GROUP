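; BP_PowerupProjectile is a projectile that delivers a powerup to players on impact.
; Tick moves it forward a fixed step per frame, ignoring delta time and without sweeping.
; Overlapping anything but its instigator triggers Detonate, which sends impact and powerup to players inside EffectTrigger.
; Detonate then spawns BP_PowerupExplosion and sets AutoDestroyWhenFinished rather than destroying itself directly.
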(event `self.ReceiveBeginPlay`)

(event `self.ReceiveTick`
  (params (DeltaSeconds :type "Float (single-precision)"))
  (`self.Fly` DeltaSeconds))

(event `self.Mesh.OnComponentBeginOverlap`
  (params (OverlappedComponent :type "PrimitiveComponent Object Reference") (OtherActor :type "Actor Object Reference") (OtherComp :type "PrimitiveComponent Object Reference") (OtherBodyIndex :type Integer) (bFromSweep :type Boolean) (SweepResult :type "HitResult Structure (by ref)"))
  (if (not (== OtherActor (`self.GetInstigator`)))
    (`self.Detonate`)))

(fn `Detonate`
  (for _array_element (`PrimitiveComponent.GetOverlappingActors` (`self.EffectTrigger`) "/Script/PrototypeTGP.FortuneFrenzyPlayer")
    (bind _asbp_player_remake (cast `/Game/Blueprint/BP_PlayerRemake` _array_element))
    (`/Game/Blueprint/BP_PlayerRemake.PowerupProjectileImpact` _asbp_player_remake (`self.GetActorForwardVector`) (`self.K2_GetActorLocation`))
    (`FortuneFrenzyPlayer.ApplyPowerup` _asbp_player_remake (`self.GetPowerup`) false))
  (`|SpawnActorFromClass` "/Game/Blueprint/BP_PowerupExplosion.BP_PowerupExplosion_C" (`self.GetTransform`) "AlwaysSpawn" "OverrideRootScale" null null)
  (set `self.bAutoDestroyWhenFinished` true))

(fn `Fly`
  (params (DeltaTime :type "Float (double-precision)"))
  (`self.K2_SetActorLocation` (* (+ (`self.K2_GetActorLocation`) (* (`self.GetActorForwardVector`) 25.0)) 1.0)))

(fn `UserConstructionScript`)