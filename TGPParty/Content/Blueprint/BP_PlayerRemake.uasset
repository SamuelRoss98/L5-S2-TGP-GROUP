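; Player actor that carries out powerup abilities and shows their status effects.
; Powerup state changes toggle particles and meshes from StatChanges modifiers, while Tick uses ForcePull to drag overlapping static mesh actors toward the player.
; Events trigger a forward blink teleport, projectiles loaded with the primary or secondary powerup from PowerupActivator, and a jittered radial burst of clones.
; Projectile impact handling only draws a debug line.
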(event `self.ReceiveBeginPlay`
  (`ActorComponent.Deactivate` (`self.SlimeParticle`))
  (`self.DeactivateSpeedEffects`)
  (`ActorComponent.Deactivate` (`self.StunParticle`))
  (`ActorComponent.Deactivate` (`self.BlinkParticle`)))

(event `self.ReceiveTick`
  (params (DeltaSeconds :type "Float (single-precision)"))
  (`self.ForcePull`))

(event `self.Teleport`
  (`self.BlinkTeleport`))

(event `self.PowerupStateChange`
  (`self.UpdatePowerupEffects`))

(event `self.FirePrimaryPowerProjectile`
  (`self.FirePowerupProjectile` true))

(event `self.FireSecondaryPowerProjectile`
  (`self.FirePowerupProjectile` false))

(event `self.SpawnClones`
  (`self.SpawnPlayerClones`))

(fn `ActivateSpeedEffects`
  (`ActorComponent.Activate` (`self.Speed Particle A`) true)
  (`ActorComponent.Activate` (`self.Speed Particle B`) true))

(fn `BlinkTeleport`
  (`self.K2_SetActorLocation` (+ (`self.K2_GetActorLocation`) (* (`self.GetActorForwardVector`) (`self.BlinkDistance`))) false true)
  (`ActorComponent.Activate` (`self.BlinkParticle`) true))

(fn `DeactivateSpeedEffects`
  (`ActorComponent.Deactivate` (`self.Speed Particle A`))
  (`ActorComponent.Deactivate` (`self.Speed Particle B`)))

(fn `FirePowerupProjectile`
  (params (Primary :type Boolean))
  (bind _firepoint (`self.FirePoint`))
  (bind _powerupactivator (`self.PowerupActivator`))
  (bind _returnvalue (`|SpawnActorFromClass` "/Game/Blueprint/BP_PowerupProjectile.BP_PowerupProjectile_C" (`KismetMathLibrary.MakeTransform` (`SceneComponent.K2_GetComponentLocation` _firepoint) (`SceneComponent.K2_GetComponentRotation` _firepoint)) "AlwaysSpawn" "OverrideRootScale" null self))
  (if Primary
    (`PowerupProjectile.SetPowerup` _returnvalue (`PowerupActivatorComponent.PrimaryPowerup` _powerupactivator))
    (else
      (`PowerupProjectile.SetPowerup` _returnvalue (`PowerupActivatorComponent.SecondaryPowerup` _powerupactivator)))))

(fn `ForcePull`
  (if (`StatModifierComponent.IsModifierActive` (`self.StatChanges`) "ForcePull")
    (for _array_element (`PrimitiveComponent.GetOverlappingActors` (`self.ForcePowerTrigger`) null)
      (bind _asstatic_mesh_actor (cast `StaticMeshActor` _array_element))
      (`PrimitiveComponent.AddForce` (`StaticMeshActor.StaticMeshComponent` _asstatic_mesh_actor) (* (`KismetMathLibrary.Normal` (- (`self.K2_GetActorLocation`) (`self.K2_GetActorLocation` _asstatic_mesh_actor))) (`StatModifierComponent.GetModifierAmount` (`self.StatChanges`) "ForcePull")) "None" false))))

(fn `PowerupProjectileImpact`
  (params (`Impact Direction` :type "Vector Structure") (`Impact Location` :type "Vector Structure"))
  (`KismetSystemLibrary.DrawDebugLine` `Impact Location` (+ (`self.K2_GetActorLocation`) (* `Impact Direction` 10000.0)) (struct :`R` 1.0 :`A` 1.0) 1.0 5.0))

(fn `SpawnPlayerClones`
  (bind _returnvalue_location (`KismetMathLibrary.BreakTransform` (`self.GetTransform`)))
  (for _index (range (+ (`self.CloneSpawnCount`) 1))
    (`|SpawnActorFromClass` "/Game/Blueprint/BP_ClonePlayer.BP_ClonePlayer_C" (`KismetMathLibrary.MakeTransform` _returnvalue_location (`KismetMathLibrary.MakeRotator` 0.0 0.0 (+ (* _index (/ 360.0 (`KismetMathLibrary.Conv_IntToDouble` (`self.CloneSpawnCount`)))) (`KismetMathLibrary.RandomFloatInRange` -15.0 15.0)))) "AlwaysSpawn" "OverrideRootScale" null null)))

(fn `UpdatePowerupEffects`
  (bind _slimeparticle (`self.SlimeParticle`))
  (bind _stunparticle (`self.StunParticle`))
  (bind _statchanges (`self.StatChanges`))
  (`SceneComponent.SetVisibility` (`self.MagetEffect`) (`StatModifierComponent.IsModifierActive` (`self.StatChanges`) "ForcePull") false)
  (if (`StatModifierComponent.IsModifierActive` (`self.StatChanges`) "Slowness")
    (`ActorComponent.Activate` _slimeparticle true)
    (else
      (`ActorComponent.Deactivate` _slimeparticle)))
  (`SceneComponent.SetVisibility` (`self.ShieldEffect`) (`StatModifierComponent.IsModifierActive` _statchanges "Invulnerability") false)
  (if (`StatModifierComponent.IsModifierActive` _statchanges "Speed")
    (`self.ActivateSpeedEffects`)
    (else
      (`self.DeactivateSpeedEffects`)))
  (if (`StatModifierComponent.IsModifierActive` (`self.StatChanges`) "Stun")
    (`ActorComponent.Activate` _stunparticle true)
    (else
      (`ActorComponent.Deactivate` _stunparticle))))

(fn `UserConstructionScript`)