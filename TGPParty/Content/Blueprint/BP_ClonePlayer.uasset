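; BP_ClonePlayer is a clone player actor that pushes itself forward using physics forces.
; On BeginPlay it picks a random walk force between configurable minimum and maximum values, so instances can differ in push strength.
; Every Tick it applies that force to its static mesh along the mesh's normalized forward vector, without steering or input handling.
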(event `self.ReceiveBeginPlay`
  (set `self.WalkForce` (`KismetMathLibrary.RandomFloatInRange` (`self.MinWalkForce`) (`self.MaxWalkForce`))))

(event `self.ReceiveTick`
  (params (DeltaSeconds :type "Float (single-precision)"))
  (`PrimitiveComponent.AddForce` (`self.StaticMesh`) (* (`KismetMathLibrary.Normal` (`SceneComponent.GetForwardVector` (`self.StaticMesh`))) (`self.WalkForce`)) "None" false))

(fn `UserConstructionScript`)