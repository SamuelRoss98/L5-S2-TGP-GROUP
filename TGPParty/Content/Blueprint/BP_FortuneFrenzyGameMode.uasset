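; BP_FortuneFrenzyGameMode is the Fortune Frenzy game mode Blueprint that sets up the on-screen powerup UI.
; On BeginPlay it creates the PowerupUI widget, adds it to the viewport, then refreshes it.
; The refresh requires player controller 0 to be a FortuneFrenzyPlayerController, but sets player one's primary power icon from a Test variable rather than that controller's data.
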(event `self.ReceiveBeginPlay`
  (`self.CreatePowerupUI`)
  (`self.RefreshPowerupUI`))

(fn `CreatePowerupUI`
  (bind _returnvalue (`|CreateWidget` "/Game/UI/PowerupUI.PowerupUI_C"))
  (bind _output_get (set `self.PowerupUI` _returnvalue))
  (`UserWidget.AddToViewport` _output_get 0))

(fn `RefreshPowerupUI`
  (bind (_test_name _test_iconpath _test_icon) (break `Powerup` (`self.Test`)))
  (bind _asfortune_frenzy_player_controller (cast `FortuneFrenzyPlayerController` (`GameplayStatics.GetPlayerController` 0)))
  (`/Game/UI/PowerupUI.SetP1PrimaryPower` (`self.PowerupUI`) _test_icon))

(fn `UserConstructionScript`)